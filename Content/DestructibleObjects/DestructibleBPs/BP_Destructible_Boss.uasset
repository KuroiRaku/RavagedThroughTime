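; BP_Destructible_Boss is a boss variant of a destructible object that faces the player and triggers a dimension switch when destroyed.
; Every Tick it rotates ObjectMesh toward the first-person character's camera using a look-at rotation.
; On death it runs the parent's death logic, then calls SwitchToDimension1 on its switcher reference.
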(event `self.ReceiveTick`
  (params (DeltaSeconds :type "Float (single-precision)"))
  (bind _asbp_first_person_character (cast `/Game/FirstPerson/Blueprints/BP_FirstPersonCharacter` (`GameplayStatics.GetPlayerCharacter` 0)))
  (`SceneComponent.K2_SetWorldRotation` (`self.ObjectMesh`) (`KismetMathLibrary.FindLookAtRotation` (`SceneComponent.K2_GetComponentLocation` (`self.ObjectMesh`)) (`SceneComponent.K2_GetComponentLocation` (`GameJamCharacter.FirstPersonCameraComponent` _asbp_first_person_character))) false false))

(event `self.OnDeath`
  (params (HitLocation :type "Vector Structure"))
  (`parent.OnDeath` HitLocation)
  (`/Game/FirstPerson/Blueprints/BP_DimensionSwitcher.SwitchToDimension1` (`self.SwitcherRef`)))

(fn `UserConstructionScript`
  (`parent.UserConstructionScript`))