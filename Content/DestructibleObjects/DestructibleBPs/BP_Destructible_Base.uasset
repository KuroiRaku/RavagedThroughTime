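; Base destructible object that loses health per hit, with a scale jiggle and health-tinted impact particles.
; A hit at zero health triggers a colored explosion, score pop-up and sound, adds points to the player, then destroys the actor.
; SwitchDimention toggles the mesh between visible-solid and hidden-overlappable, or destroys it if health is depleted.
; When the player's capsule overlaps the mesh, a delayed recursive check postpones making it solid until clear.
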(event `self.ReceiveTick`
  (params (DeltaSeconds :type "Float (single-precision)")))

(event `OnDeath`
  (params (HitLocation :type "Vector Structure"))
  (`/Engine/EditorBlueprintResources/StandardMacros.DoOnce` false
    (:`Completed`
      (`self.Object Exploded` HitLocation)
      (bind _asbp_first_person_character (cast `/Game/FirstPerson/Blueprints/BP_FirstPersonCharacter` (`GameplayStatics.GetPlayerCharacter` 0)))
      (set `/Game/FirstPerson/Blueprints/BP_FirstPersonCharacter.CurrentPoints` (+ (`/Game/FirstPerson/Blueprints/BP_FirstPersonCharacter.CurrentPoints` _asbp_first_person_character) (`self.PointsAwarded`)) _asbp_first_person_character)
      (`GameplayStatics.SpawnSoundAtLocation` (`self.ExplosionSound`) HitLocation (struct) 1.0 1.0 0.0 null null)
      (`self.K2_DestroyActor`))))

(event `self.ReceiveBeginPlay`
  (set `self.CurrentHealth` (`KismetMathLibrary.Conv_IntToDouble` (`self.MaxHealth`)))
  (set `self.DefaultMeshScale` (`SceneComponent.K2_GetComponentScale` (`self.ObjectMesh`))))

(event `OnHitJiggle`
  (bind _defaultmeshscale (`self.DefaultMeshScale`))
  (bind _objectmesh (`self.ObjectMesh`))
  (bind (_direction _amount) (`Timeline|Jiggle` :!via `PlayFromStart`)
    (:`Update`
      (`/Engine/EditorBlueprintResources/StandardMacros.IsValid` _objectmesh
        (:`Is Valid`
          (`SceneComponent.SetWorldScale3D` _objectmesh (`KismetMathLibrary.VLerp` _defaultmeshscale (* _defaultmeshscale 0.95) _amount)))))))

(event `CheckForOverlap`
  (bind _objectmesh (`self.ObjectMesh`))
  (`KismetSystemLibrary.Delay` 0.01)
  (bind _asbp_first_person_character (cast `/Game/FirstPerson/Blueprints/BP_FirstPersonCharacter` (`GameplayStatics.GetPlayerCharacter` 0)))
  (if (not (`PrimitiveComponent.IsOverlappingComponent` (`Character.CapsuleComponent` _asbp_first_person_character) _objectmesh))
    (if (not (`/Game/FirstPerson/Blueprints/BP_DimensionSwitcher.InDimension2` (`self.SwitcherRef`)))
      (`SceneComponent.SetVisibility` _objectmesh true true)
      (`PrimitiveComponent.SetCollisionEnabled` _objectmesh "QueryAndPhysics")
      (`PrimitiveComponent.SetCollisionResponseToChannel` _objectmesh "ECC_Pawn" "ECR_Block")
      (`PrimitiveComponent.SetCollisionResponseToChannel` _objectmesh "ECC_Visibility" "ECR_Block"))
    (else
      (`self.CheckForOverlap`))))

(fn `Object Exploded`
  (params (HitLocation :type "Vector Structure"))
  (`|ExecutionSequence`
    (:`then_0`
      (bind _returnvalue (`NiagaraFunctionLibrary.SpawnSystemAtLocation` "/Game/Particles/NS_ObjectExplosion.NS_ObjectExplosion" HitLocation (struct) (`SceneComponent.K2_GetComponentScale` (`self.DefaultSceneRoot`))))
      (`NiagaraComponent.SetVariableLinearColor` _returnvalue "ParticleColourMax" (`self.ParticleColourMax`))
      (`NiagaraComponent.SetVariableLinearColor` _returnvalue "ParticleColourMin" (`self.ParticleColourMin`))
      (bind _returnvalue_2 (`|SpawnActorFromClass` "/Game/DestructibleObjects/Other/BP_ScorePopUp.BP_ScorePopUp_C" (`KismetMathLibrary.MakeTransform` (`local.HitLocation`) (struct) (`KismetMathLibrary.Conv_DoubleToVector` (`KismetMathLibrary.Lerp` 0.6 3.0 (/ (`KismetMathLibrary.Conv_IntToDouble` (`self.PointsAwarded`)) 25.0)))) "Undefined" "OverrideRootScale" null null))
      (bind _asw_score_pop_up (cast `/Game/DestructibleObjects/Other/W_ScorePopUp` (`WidgetComponent.GetWidget` (`/Game/DestructibleObjects/Other/BP_ScorePopUp.Widget` _returnvalue_2))))
      (set `/Game/DestructibleObjects/Other/W_ScorePopUp.BaseColour` (`self.ParticleColourMin`) _asw_score_pop_up)
      (set `/Game/DestructibleObjects/Other/W_ScorePopUp.OutlineColour` (`self.ParticleColourMax`) _asw_score_pop_up)
      (set `/Game/DestructibleObjects/Other/W_ScorePopUp.ScoreToShow` (`self.PointsAwarded`) _asw_score_pop_up))
    (:`then_1`
      (`ActorComponent.K2_DestroyComponent` (`self.ObjectMesh`)))))

(fn `OnHit`
  (params (HitLocation :type "Vector Structure"))
  (if (<= (`self.CurrentHealth`) 0.0)
    (`/Engine/EditorBlueprintResources/StandardMacros.DoOnce` false
      (:`Completed`
        (`self.OnDeath` HitLocation)))
    (else
      (set `self.CurrentHealth` (- (`self.CurrentHealth`) 1.0))
      (`self.SpawnHitParticles` HitLocation)
      (`self.OnHitJiggle`))))

(fn `SpawnHitParticles`
  (params (HitLocation :type "Vector Structure"))
  (bind _returnvalue (`NiagaraFunctionLibrary.SpawnSystemAtLocation` "/Game/Particles/NS_HitImpact.NS_HitImpact" HitLocation))
  (`NiagaraComponent.SetVariableLinearColor` _returnvalue "ParticleColour" (`KismetMathLibrary.LinearColorLerp` (struct :`R` 1.0 :`B` 0.1 :`A` 1.0) (struct :`R` 0.5 :`G` 1.0 :`A` 1.0) (/ (`self.CurrentHealth`) (`self.MaxHealth`)))))

(fn `SwitchDimention`
  (params (InDimention2 :type Boolean))
  (bind _objectmesh (`self.ObjectMesh`))
  (if (> (`self.CurrentHealth`) 0.0)
    (if InDimention2
      (bind _asbp_first_person_character (cast `/Game/FirstPerson/Blueprints/BP_FirstPersonCharacter` (`GameplayStatics.GetPlayerCharacter` 0)))
      (if (not (`PrimitiveComponent.IsOverlappingComponent` (`Character.CapsuleComponent` _asbp_first_person_character) _objectmesh))
        (`SceneComponent.SetVisibility` _objectmesh true true)
        (`PrimitiveComponent.SetCollisionEnabled` _objectmesh "QueryAndPhysics")
        (`PrimitiveComponent.SetCollisionResponseToChannel` _objectmesh "ECC_Pawn" "ECR_Block")
        (`PrimitiveComponent.SetCollisionResponseToChannel` _objectmesh "ECC_Visibility" "ECR_Block")
        (else
          (`self.CheckForOverlap`)))
      (else
        (`SceneComponent.SetVisibility` _objectmesh false true)
        (`PrimitiveComponent.SetCollisionEnabled` _objectmesh "QueryOnly")
        (`PrimitiveComponent.SetCollisionResponseToChannel` _objectmesh "ECC_Pawn" "ECR_Overlap")
        (`PrimitiveComponent.SetCollisionResponseToChannel` _objectmesh "ECC_Visibility" "ECR_Ignore")))
    (else
      (`self.K2_DestroyActor`))))

(fn `UserConstructionScript`)