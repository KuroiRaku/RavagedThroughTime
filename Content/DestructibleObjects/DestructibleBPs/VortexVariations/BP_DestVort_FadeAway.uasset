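; Destructible vortex variation that fades away by shrinking its mesh to nothing.
; On BeginPlay and after each dimension switch, RestartShrink activates the vortex smoke and plays a timeline that lerps the mesh from its starting scale to zero, then deactivates the smoke.
; The construction script tints a dynamic material instance with the minimum particle colour.
; OnHitJiggle is an empty event.
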(event `self.ReceiveBeginPlay`
  (`parent.ReceiveBeginPlay`)
  (set `self.StartingScale` (`SceneComponent.K2_GetComponentScale` (`self.ObjectMesh`)))
  (`self.RestartShrink`))

(event `RestartShrink`
  (bind _objectmesh (`self.ObjectMesh`))
  (`ActorComponent.SetActive` (`self.NS_VortexSmoke`) true false)
  (bind (_direction _newtrack_0) (`Timeline|Shrinking` :!via `PlayFromStart`)
    (:`Update`
      (`/Engine/EditorBlueprintResources/StandardMacros.IsValid` _objectmesh
        (:`Is Valid`
          (`SceneComponent.SetWorldScale3D` _objectmesh (`KismetMathLibrary.VLerp` (`self.StartingScale`) (0.0 0.0 0.0) _newtrack_0)))))
    (:`Finished`
      (`ActorComponent.Deactivate` (`self.NS_VortexSmoke`)))))

(event `self.OnHitJiggle`)

(fn `SwitchDimention`
  (params (InDimention2 :type Boolean))
  (`parent.SwitchDimention` InDimention2)
  (if true
    (`self.RestartShrink`)))

(fn `UserConstructionScript`
  (`parent.UserConstructionScript`)
  (bind _returnvalue (`KismetMaterialLibrary.CreateDynamicMaterialInstance` (`PrimitiveComponent.GetMaterial` (`self.ObjectMesh`) 0)))
  (`MaterialInstanceDynamic.SetVectorParameterValue` _returnvalue "VortexMainColour" (`self.ParticleColourMin`))
  (`PrimitiveComponent.SetMaterial` (`self.ObjectMesh`) 0 _returnvalue))