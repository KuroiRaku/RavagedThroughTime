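; Moving variant of a destructible vortex object that carries its mesh along a spline.
; A timeline with play rate 1/Speed samples the spline each update and teleports ObjectMesh to that location and rotation, keeping its scale.
; On finish it restarts from the start when IsLooping is set, otherwise it ping-pongs by reversing.
; The construction script tints a dynamic material's VortexMainColour with ParticleColourMin.
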(event `self.ReceiveBeginPlay`
  (`parent.ReceiveBeginPlay`)
  (`TimelineComponent.SetPlayRate` (`self.Timeline_0`) (/ 1.0 (`self.Speed`)))
  (`self.StartMovement`))

(event `StartMovement`
  (bind _objectmesh (`self.ObjectMesh`))
  (bind (_direction _amount) (`Timeline|Timeline_0` :!via `PlayFromStart` :!label _label)
    (:`Update`
      (`/Engine/EditorBlueprintResources/StandardMacros.IsValid` _objectmesh
        (:`Is Valid`
          (bind (_returnvalue_location _returnvalue_rotation) (`KismetMathLibrary.BreakTransform` (`SplineComponent.GetTransformAtTime` (`self.Spline`) _amount "World" false false)))
          (`SceneComponent.K2_SetWorldTransform` _objectmesh (`KismetMathLibrary.MakeTransform` _returnvalue_location _returnvalue_rotation (`SceneComponent.K2_GetComponentScale` (`self.ObjectMesh`))) false true))))
    (:`Finished`
      (if (`self.IsLooping`)
        (`self.StartMovement`)
        (elif (== _amount 1.0)
          (`self.RevertMovement`)
          (else
            (`self.StartMovement`)))))))

(event `RevertMovement`
  (goto _label :!via `Reverse`))

(fn `UserConstructionScript`
  (`parent.UserConstructionScript`)
  (bind _returnvalue (`KismetMaterialLibrary.CreateDynamicMaterialInstance` (`PrimitiveComponent.GetMaterial` (`self.ObjectMesh`) 0)))
  (`MaterialInstanceDynamic.SetVectorParameterValue` _returnvalue "VortexMainColour" (`self.ParticleColourMin`))
  (`PrimitiveComponent.SetMaterial` (`self.ObjectMesh`) 0 _returnvalue))