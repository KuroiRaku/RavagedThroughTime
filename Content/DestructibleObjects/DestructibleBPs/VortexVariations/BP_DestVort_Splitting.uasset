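; Splitting variant of a destructible vortex that breaks into smaller vortices when destroyed.
; On death it runs the parent logic, then spawns a scaled-down BP_Destructible_Vortex at each of three spawn point components, overriding their health and points awarded.
; The construction script gives the mesh a dynamic material tinted by the minimum particle colour.
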(event `self.OnDeath`
  (params (HitLocation :type "Vector Structure"))
  (`parent.OnDeath` HitLocation)
  (for _array_element (`|MakeArray` (`self.SpawnPoint2`) (`self.SpawnPoint3`) (`self.SpawnPoint1`))
    (`|SpawnActorFromClass` "/Game/DestructibleObjects/DestructibleBPs/BP_Destructible_Vortex.BP_Destructible_Vortex_C" (`KismetMathLibrary.MakeTransform` (`SceneComponent.K2_GetComponentLocation` _array_element) (struct) (0.3 0.3 0.3)) "Undefined" "OverrideRootScale" null 3 8 null null)))

(fn `UserConstructionScript`
  (`parent.UserConstructionScript`)
  (bind _returnvalue (`KismetMaterialLibrary.CreateDynamicMaterialInstance` (`PrimitiveComponent.GetMaterial` (`self.ObjectMesh`) 0)))
  (`MaterialInstanceDynamic.SetVectorParameterValue` _returnvalue "VortexMainColour" (`self.ParticleColourMin`))
  (`PrimitiveComponent.SetMaterial` (`self.ObjectMesh`) 0 _returnvalue))