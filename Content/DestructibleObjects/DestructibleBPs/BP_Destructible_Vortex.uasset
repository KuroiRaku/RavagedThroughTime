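; BP_Destructible_Vortex is a destructible object with a vortex smoke Niagara effect that awards points to the player when destroyed.
; The construction script tints the smoke particles with its minimum particle colour.
; On death it calls ObjectExploded at the hit location and deactivates the smoke.
; If the player is a BP_FirstPersonCharacter, it then adds points, plays an explosion sound and destroys itself after a short delay.
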(event `self.ReceiveBeginPlay`
  (`parent.ReceiveBeginPlay`))

(event `self.OnDeath`
  (params (HitLocation :type "Vector Structure"))
  (`self.Object Exploded` HitLocation)
  (`ActorComponent.Deactivate` (`self.NS_VortexSmoke`))
  (bind _asbp_first_person_character (cast `/Game/FirstPerson/Blueprints/BP_FirstPersonCharacter` (`GameplayStatics.GetPlayerCharacter` 0)))
  (set `/Game/FirstPerson/Blueprints/BP_FirstPersonCharacter.CurrentPoints` (+ (`/Game/FirstPerson/Blueprints/BP_FirstPersonCharacter.CurrentPoints` _asbp_first_person_character) (`self.PointsAwarded`)) _asbp_first_person_character)
  (`GameplayStatics.SpawnSoundAtLocation` (`self.ExplosionSound`) HitLocation (struct) 1.0 1.0 0.0 null null)
  (`KismetSystemLibrary.Delay` 4.0)
  (`self.K2_DestroyActor`))

(fn `UserConstructionScript`
  (`parent.UserConstructionScript`)
  (`NiagaraComponent.SetVariableLinearColor` (`self.NS_VortexSmoke`) "ParticlesColour" (`self.ParticleColourMin`)))