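; BP_ScorePopUp is a short-lived actor, named as a score pop-up, that shows a widget in the world and removes itself after a brief delay.
; Each Tick, it rotates the Widget component to face the first-person character's camera using a look-at rotation.
; The same Tick moves the actor upward by a fixed step per frame, so the rise speed depends on frame rate.
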(event `self.ReceiveBeginPlay`
  (`KismetSystemLibrary.Delay` 2.5)
  (`self.K2_DestroyActor`))

(event `self.ReceiveTick`
  (params (DeltaSeconds :type "Float (single-precision)"))
  (bind _widget (`self.Widget`))
  (`|ExecutionSequence`
    (:`then_0`
      (bind _asbp_first_person_character (cast `/Game/FirstPerson/Blueprints/BP_FirstPersonCharacter` (`GameplayStatics.GetPlayerCharacter` 0)))
      (`SceneComponent.K2_SetWorldRotation` _widget (`KismetMathLibrary.FindLookAtRotation` (`SceneComponent.K2_GetComponentLocation` _widget) (`SceneComponent.K2_GetComponentLocation` (`GameJamCharacter.FirstPersonCameraComponent` _asbp_first_person_character))) false false))
    (:`then_1`
      (`self.K2_SetActorLocation` (+ (`self.K2_GetActorLocation`) (0.0 0.0 0.3))))))

(fn `UserConstructionScript`)